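; BP_Door is a sliding door that opens only while all of its linked pressure plates are pressed.
; On BeginPlay it binds to each plate's pressed and released events, which maintain a running count.
; When the count equals the number of plates, the mesh moves up via MoveComponentTo and the OnOpened dispatcher fires.
; Releasing any plate while open lowers it again, with no matching closed event.
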(event Custom|PlatePressed
  (bind _output_get (Variables|Default|SetPressedCount (+ (Variables|Default|GetPressedCount) 1)))
  (if (== _output_get (Utilities|Array|Length (Variables|Default|GetPlates)))
    (CallFunction|OpenDoor)))

(event Custom|PlateReleased
  (Variables|Default|SetPressedCount (- (Variables|Default|GetPressedCount) 1))
  (if (Variables|Default|GetbOpen)
    (CallFunction|CloseDoor)))

(event Custom|OpenDoor
  (Variables|Default|SetbOpen true)
  (Components|MoveComponentTo (Variables|Default|GetDoorMesh) (Math|Vector|MakeVector 0.0 0.0 4.6e+02) "0, 0, 0" false false 1.0 false)
  (Default|CallOnOpened))

(event Custom|CloseDoor
  (Variables|Default|SetbOpen false)
  (Components|MoveComponentTo (Variables|Default|GetDoorMesh) (Math|Vector|MakeVector 0.0 0.0 1.5e+02) "0, 0, 0" false false 1.0 false))

(event EventBeginPlay
  (for _array_element (Variables|Default|GetPlates)
    (EventDispatchers|BindEventtoOnPlatePressed _array_element (delegate Custom|PlatePressed))
    (EventDispatchers|BindEventtoOnPlateReleased _array_element (delegate Custom|PlateReleased))))

(event Collision|EventActorBeginOverlap
  (params (OtherActor :type Actor%20Object%20Reference)))

(event EventTick
  (params (DeltaSeconds :type Float%20%28single-precision%29)))

(fn ConstructionScript)