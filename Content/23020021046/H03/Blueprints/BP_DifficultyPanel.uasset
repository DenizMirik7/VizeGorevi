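; BP_DifficultyPanel lets the player choose one of four difficulty levels with number keys 1 to 4.
; It enables player input on BeginPlay, then each key calls ApplyDifficulty, which stores the level and prints its Turkish name and enemy count.
; EnemyCountFor separately maps a level to an enemy count through a Select, but nothing in this Blueprint calls it or spawns enemies.
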(event EventBeginPlay
  (Input|EnableInput (Game|GetPlayerController 0)))

(event Input|KeyboardEvents|1
  (params (Key :type Key%20Structure))
  (:Pressed
    (CallFunction|ApplyDifficulty)))

(event Input|KeyboardEvents|2
  (params (Key :type Key%20Structure))
  (:Pressed
    (CallFunction|ApplyDifficulty 1)))

(event Input|KeyboardEvents|3
  (params (Key :type Key%20Structure))
  (:Pressed
    (CallFunction|ApplyDifficulty 2)))

(event Input|KeyboardEvents|4
  (params (Key :type Key%20Structure))
  (:Pressed
    (CallFunction|ApplyDifficulty 3)))

(fn ConstructionScript)

(fn ApplyDifficulty
  (params (Level :type Integer))
  (Variables|Default|SetDifficulty Level)
  (switch int Level
    (:Default
      (Development|PrintString "Geçersiz zorluk!"))
    (:0
      (Development|PrintString "Kolay: 5 düşman"))
    (:1
      (Development|PrintString "Normal: 10 düşman"))
    (:2
      (Development|PrintString "Zor: 15 düşman"))
    (:3
      (Development|PrintString "Kâbus: 25 düşman"))))

(fn EnemyCountfor
  (params (Level :type Integer))
  (return (Utilities|Select :Index Level :Option%200 5 :Option%201 10 :Option%202 15 :Option%203 25)))