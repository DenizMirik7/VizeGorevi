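; BP_H03_Ornekler is a collection of small Blueprint examples, each in its own function or event, reporting mostly through printed messages in Turkish.
; BeginPlay contrasts a delayed and an immediate Sequence branch, while a separate event starts a looping countdown timer with no stop condition.
; Independent functions demonstrate array searches with and without break, string switching, text formatting, type conversions, a math-expression damage formula, interpolation, range mapping and dice rolls.
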(event Custom|StartCountdown
  (Utilities|Time|SetTimerbyEvent (delegate Custom|Countdown) 1.0 true))

(event Custom|Countdown
  (bind _output_get (Variables|Default|SetTimeLeft (- (Variables|Default|GetTimeLeft) 1)))
  (Development|PrintString (Utilities|String|Append "Kalan süre: " (Utilities|String|ToString(Integer) _output_get))))

(event EventBeginPlay
  (Utilities|FlowControl|Sequence
    (:then_0
      (Utilities|FlowControl|Delay 2.0)
      (Development|PrintString "Then 0: Delay bitti (2 sn sonra)"))
    (:then_1
      (Development|PrintString "Then 1: Beklemeden çalıştı"))))

(fn ConstructionScript)

(fn FindBestScore
  (Variables|Default|SetBestScore 0.0)
  (for (_array_element _array_index) (Variables|Default|GetScores)
    (if (> _array_element (Variables|Default|GetBestScore))
      (Variables|Default|SetBestScore _array_element)
      (Variables|Default|SetBestPlayer _array_index)))
  (Development|PrintString (Utilities|String|Append "Kazanan: Oyuncu " (Utilities|String|ToString(Integer) (Variables|Default|GetBestPlayer)))))

(fn FindItem
  (params (ItemName :type String))
  (Variables|Default|SetFoundIndex -1)
  (bind (_array_element _array_index) (Utilities|Array|ForEachLoopwithBreak (Variables|Default|GetInventory) :!label _label)
    (:LoopBody
      (if (Utilities|Enum|Equal(Enum) _array_element ItemName)
        (Variables|Default|SetFoundIndex _array_index)
        (goto _label Break)))
    (:Completed
      (Development|PrintString (Utilities|String|Append "Bulunan index: " (Utilities|String|ToString(Integer) (Variables|Default|GetFoundIndex)))))))

(fn RunCheat
  (params (Command :type String))
  (switch string (Utilities|String|ToLower Command)
    (:Default
      (Development|PrintString "Bilinmeyen komut"))
    (:god
      (Development|PrintString "Ölümsüzlük açık"))
    (:fly
      (Development|PrintString "Uçma modu açık"))
    (:heal
      (Development|PrintString "Can dolduruldu"))))

(fn Welcome
  (params (PlayerName :type String))
  (Development|PrintString (Utilities|String|Append "Hoş geldin, " PlayerName "!")))

(fn MatchResult
  (params (Oyuncu1 :type String) (Skor1 :type Integer) (Oyuncu2 :type String) (Skor2 :type Integer))
  (Development|PrintText (Utilities|Text|FormatText "Sonuç: {Oyuncu1} = {Skor1} X {Oyuncu2} = {Skor2}" Oyuncu1 Skor1 Oyuncu2 Skor2)))

(fn Conversions
  (Development|PrintString (Utilities|String|ToString(Integer) (* (Math|Conversions|ToInteger(Byte) "150") 2)))
  (Development|PrintText (Utilities|Text|ToText(Float) 3.14159 "HalfToEven" false true 1 324 0 2)))

(fn CalculateAttackDamage
  (params (BaseWeaponDamage :type Float%20%28double-precision%29) (AbilityModifier :type Float%20%28double-precision%29) (Enhancement :type Float%20%28double-precision%29) (CurrentStatus :type Float%20%28double-precision%29))
  (return (|(((BaseWeaponDamage+AbilityModifier)+Enhancement)*CurrentStatus) BaseWeaponDamage AbilityModifier Enhancement CurrentStatus)))

(fn RaceProgress
  (params (Alpha :type Float%20%28double-precision%29))
  (return (Math|Float|Lerp 1.5e+03 9.5e+03 Alpha)))

(fn AmmoPercent
  (params (Ammo :type Float%20%28double-precision%29))
  (return (Math|Float|MapRangeClamped Ammo 0.0 3e+01 0.0 1e+02)))

(fn RollDiceDogru
  (LocalVariables|SetDice (Math|Random|RandomIntegerinRange 1 6))
  (Development|PrintString (Utilities|String|Append "Zar: " (Utilities|String|ToString(Integer) (LocalVariables|GetDice))))
  (if (== (LocalVariables|GetDice) 6)
    (Development|PrintString "Altı geldi!")))