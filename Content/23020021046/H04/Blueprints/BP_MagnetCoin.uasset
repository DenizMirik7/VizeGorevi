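; BP_MagnetCoin is a collectible coin that spins and pulls itself toward the player.
; Each tick it rotates on yaw and, when the player character is within PullRadius, moves straight toward them at Speed, capping the step so it never overshoots.
; Overlapping any Character prints a Turkish "coin collected" message and destroys the coin, without adding to any score.
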(event EventTick
  (params (DeltaSeconds :type Float%20%28single-precision%29))
  (bind _returnvalue (Game|GetPlayerCharacter 0))
  (bind _returnvalue_2 (Transformation|GetActorLocation))
  (bind _returnvalue_3 (Transformation|GetDistanceTo _returnvalue))
  (Transformation|AddActorLocalRotation (Math|Rotator|MakeRotator 0.0 0.0 (* DeltaSeconds 1.8e+02)) false false)
  (if (< _returnvalue_3 (Variables|Default|GetPullRadius))
    (Transformation|SetActorLocation (+ _returnvalue_2 (* (Math|Vector|GetUnitDirection(Vector) _returnvalue_2 (Transformation|GetActorLocation _returnvalue)) (Math|Float|Min(Float) (* (Variables|Default|GetSpeed) DeltaSeconds) _returnvalue_3))) false false)))

(event Collision|EventActorBeginOverlap
  (params (OtherActor :type Actor%20Object%20Reference))
  (Utilities|Casting|CastToCharacter OtherActor)
  (Development|PrintString "Coin toplandı!")
  (Actor|DestroyActor))

(fn ConstructionScript)