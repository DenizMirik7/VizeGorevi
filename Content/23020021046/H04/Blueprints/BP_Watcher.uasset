(event EventTick
  (params (DeltaSeconds :type Float%20%28single-precision%29))
  (Class|KismetSystemLibrary|DrawDebugConeinDegrees (+ (Transformation|GetActorLocation) (Math|Vector|MakeVector 0.0 0.0 185.0)) (Transformation|GetActorForwardVector) (Variables|Default|GetViewDistance) 45.0 45.0 24 "(R=1.000000,G=1.000000,B=0.000000,A=1.000000)" 0.0 1.5 "World")
  (bind _seen (CallFunction|CanSeePlayer))
  (if _seen
    (Rendering|Material|SetMaterial (Variables|Default|GetBody) 0 "/Game/23020021046/H04/Materials/MI_WatcherAlert.MI_WatcherAlert")
    (Development|PrintString "GÖRÜLDÜN!" true true "(R=1.000000,G=0.000000,B=0.000000,A=1.000000)" 0.0 "Gozcu")
    (else
      (Rendering|Material|SetMaterial (Variables|Default|GetBody) 0 "/Game/23020021046/H04/Materials/MI_WatcherCalm.MI_WatcherCalm"))))

(fn ConstructionScript)

(fn CanSeePlayer
  (bind _returnvalue (Game|GetPlayerCharacter 0))
  (bind _output_get (Variables|Default|SetDotValue (Math|Vector|DotProduct (Transformation|GetActorForwardVector) (Math|Vector|GetUnitDirection(Vector) (Transformation|GetActorLocation) (Transformation|GetActorLocation _returnvalue)))))
  (return (and (< (Transformation|GetDistanceTo _returnvalue) (Variables|Default|GetViewDistance)) (> _output_get (Variables|Default|GetConeDot)))))