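; BP_Mover is an actor that shuttles back and forth along the forward axis it has at BeginPlay.
; Each tick it offsets itself along that direction by Speed scaled by delta time, without sweeping for collision.
; Once it is more than 600 units from its stored start location, it negates the direction and stores the current location as the new start for the next leg.
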(event EventBeginPlay
  (Variables|Default|SetStartLocation (Transformation|GetActorLocation))
  (Variables|Default|SetDirection (Transformation|GetActorForwardVector)))

(event EventTick
  (params (DeltaSeconds :type Float%20%28single-precision%29))
  (Transformation|AddActorWorldOffset (* (Variables|Default|GetDirection) (* (Variables|Default|GetSpeed) DeltaSeconds)))
  (if (> (Math|Vector|VectorLength (- (Transformation|GetActorLocation) (Variables|Default|GetStartLocation))) 6e+02)
    (Variables|Default|SetDirection (* (Variables|Default|GetDirection) (Math|Vector|MakeVector -1.0 -1.0 -1.0)))
    (Variables|Default|SetStartLocation (Transformation|GetActorLocation))))

(fn ConstructionScript)