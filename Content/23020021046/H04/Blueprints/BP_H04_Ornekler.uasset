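; BP_H04_Ornekler is a teaching example actor for vector math, spawning and null-safe references.
; On BeginPlay it enables player input, then prints vector addition, subtraction, length and normalization, plus dot products for same, perpendicular and opposite directions.
; T spawns a BP_PowerPill ahead of the player character along its forward vector.
; N prints Target's location unguarded, while M checks IsValid first and prints a Turkish warning when it is empty.
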(event EventBeginPlay
  (Input|EnableInput (Game|GetPlayerController 0))
  (CallFunction|VectorMath)
  (CallFunction|DotDemo))

(event Input|KeyboardEvents|T
  (params (Key :type Key%20Structure))
  (:Pressed
    (CallFunction|SpawninFront)))

(event Input|KeyboardEvents|N
  (params (Key :type Key%20Structure))
  (:Pressed
    (CallFunction|PrintTargetHatali)))

(event Input|KeyboardEvents|M
  (params (Key :type Key%20Structure))
  (:Pressed
    (CallFunction|PrintTargetGuvenli)))

(fn ConstructionScript)

(fn VectorMath
  (bind _returnvalue (Math|Vector|MakeVector 12.0 0.0 14.0))
  (bind _returnvalue_2 (Math|Vector|MakeVector 4.0 0.0 8.0))
  (bind _returnvalue_3 (- _returnvalue _returnvalue_2))
  (Development|PrintString (Utilities|String|Append "Toplama: " (Utilities|String|ToString(Vector) (+ (Math|Vector|MakeVector 5.0 0.0 9.0) (Math|Vector|MakeVector 4.0 0.0 2.0)))))
  (Development|PrintString (Utilities|String|Append "B - A: " (Utilities|String|ToString(Vector) _returnvalue_3)))
  (Development|PrintString (Utilities|String|Append "Uzunluk: " (Utilities|String|ToString(Float) (Math|Vector|VectorLength _returnvalue_3))))
  (Development|PrintString (Utilities|String|Append "Normalize: " (Utilities|String|ToString(Vector) (Math|Vector|Normalize _returnvalue_3)))))

(fn DotDemo
  (bind _returnvalue (Math|Vector|MakeVector 1.0 0.0 0.0))
  (Development|PrintString (Utilities|String|Append "Aynı yön: " (Utilities|String|ToString(Float) (Math|Vector|DotProduct _returnvalue (Math|Vector|MakeVector 1.0 0.0 0.0)))))
  (Development|PrintString (Utilities|String|Append "Dik: " (Utilities|String|ToString(Float) (Math|Vector|DotProduct _returnvalue (Math|Vector|MakeVector 0.0 1.0 0.0)))))
  (Development|PrintString (Utilities|String|Append "Zıt: " (Utilities|String|ToString(Float) (Math|Vector|DotProduct _returnvalue (Math|Vector|MakeVector -1.0 0.0 0.0))))))

(fn SpawninFront
  (bind _returnvalue (Game|GetPlayerCharacter 0))
  (Game|SpawnActorfromClass "/Game/23020021046/H04/Blueprints/BP_PowerPill.BP_PowerPill_C" (Math|Transform|MakeTransform (+ (Transformation|GetActorLocation _returnvalue) (* (Transformation|GetActorForwardVector _returnvalue) (Math|Vector|MakeVector 2e+02 2e+02 2e+02)))) "AlwaysSpawn" "MultiplyWithRoot" 0 0))

(fn PrintTargetHatali
  (Development|PrintString (Utilities|String|ToString(Vector) (Transformation|GetActorLocation (Variables|Default|GetTarget)))))

(fn PrintTargetGuvenli
  (bind _target (Variables|Default|GetTarget))
  (Utilities|IsValid _target
    (:Is%20Valid
      (Development|PrintString (Utilities|String|ToString(Vector) (Transformation|GetActorLocation _target))))
    (:Is%20Not%20Valid
      (Development|PrintString "Target boş (None)! Önce bir actor atayın."))))