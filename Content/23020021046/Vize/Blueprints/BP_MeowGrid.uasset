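; BP_MeowGrid runs a five-level cat-placement logic puzzle with one cat per row, column and color region, none touching.
; MeowLoadLevel picks the level's regions and solution, moves the camera and spawns a BP_MeowBlock grid.
; Clicks are checked for rule conflicts, then against the stored solution; mistakes cost lives, while correct cats score and auto-X neighbors.
; Hints place solution cats, W_MeowHUD shows status, and completing a level loads the next.
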(event Custom|MeowOnLevelCompleted
  (bind _hud (Variables|Default|GetHud))
  (Variables|Default|SetIsTransitioning true)
  (Variables|Default|SetScore (+ (Variables|Default|GetScore) (Class|KismetSystemLibrary|MakeLiteralInteger 50)))
  (if (< (Variables|Default|GetCurrentLevel) (Class|KismetSystemLibrary|MakeLiteralInteger 5))
    (Rendering|Components|TextRender|SetText (Variables|/Game/23020021046/Vize/UI/W_MeowHUD.W_MeowHUD_C|GettxtBanner _hud) (Utilities|Text|ToText(String) "TEBRİKLER! SEVİYE TAMAMLANDI! (+50 Puan)"))
    (Widget|SetVisibility (Variables|/Game/23020021046/Vize/UI/W_MeowHUD.W_MeowHUD_C|GettxtBanner _hud) "Visible")
    (Variables|Default|SetStatusMessage "Harika iş! Sonraki seviye 2 saniye içinde yükleniyor...")
    (CallFunction|MeowUpdateHud)
    (Utilities|FlowControl|Delay 2.2)
    (CallFunction|MeowLoadLevel (+ (Variables|Default|GetCurrentLevel) (Class|KismetSystemLibrary|MakeLiteralInteger 1)))
    (else
      (Variables|Default|SetIsGameOver true)
      (Rendering|Components|TextRender|SetText (Variables|/Game/23020021046/Vize/UI/W_MeowHUD.W_MeowHUD_C|GettxtBanner _hud) (Utilities|Text|ToText(String) "TEBRİKLER! TÜM SEVİYELER TAMAMLANDI!"))
      (Widget|SetVisibility (Variables|/Game/23020021046/Vize/UI/W_MeowHUD.W_MeowHUD_C|GettxtBanner _hud) "Visible")
      (Variables|Default|SetStatusMessage "5/5 Seviyeyi de başarıyla tamamladın! Tekrar oynamak için 1-5 veya R tuşuna basabilirsin.")
      (CallFunction|MeowUpdateHud))))

(event Custom|MeowTriggerGameOver
  (bind _hud (Variables|Default|GetHud))
  (Variables|Default|SetIsGameOver true)
  (Rendering|Components|TextRender|SetText (Variables|/Game/23020021046/Vize/UI/W_MeowHUD.W_MeowHUD_C|GettxtBanner _hud) (Utilities|Text|ToText(String) "CAN KALMADI! (R ile Yeniden Dene)"))
  (Widget|SetVisibility (Variables|/Game/23020021046/Vize/UI/W_MeowHUD.W_MeowHUD_C|GettxtBanner _hud) "Visible")
  (CallFunction|MeowUpdateHud))

(event EventBeginPlay
  (bind _returnvalue (UserInterface|CreateWidget "/Game/23020021046/Vize/UI/W_MeowHUD.W_MeowHUD_C" (Game|GetPlayerController 0)))
  (Variables|Default|SetHud _returnvalue)
  (UserInterface|Viewport|AddtoViewport _returnvalue 0)
  (CallFunction|MeowLoadLevel 1))

(event Collision|EventActorBeginOverlap
  (params (OtherActor :type Actor%20Object%20Reference)))

(event EventTick
  (params (DeltaSeconds :type Float%20%28single-precision%29)))

(fn ConstructionScript)

(fn MeowSetHoveredBlock
  (params (InBlock :type BP%20Meow%20Block%20Object%20Reference))
  (Variables|Default|SetHoveredBlock InBlock))

(fn MeowonTileLeftClicked
  (params (ClickedBlock :type BP%20Meow%20Block%20Object%20Reference))
  (bind _row (Variables|/Game/23020021046/Vize/Blueprints/BP_MeowBlock.BP_MeowBlock_C|GetRow ClickedBlock))
  (bind _col (Variables|/Game/23020021046/Vize/Blueprints/BP_MeowBlock.BP_MeowBlock_C|GetCol ClickedBlock))
  (if (not (or (Variables|Default|GetIsGameOver) (Variables|Default|GetIsTransitioning)))
    (if (== (Variables|/Game/23020021046/Vize/Blueprints/BP_MeowBlock.BP_MeowBlock_C|GetCellState ClickedBlock) (Class|KismetSystemLibrary|MakeLiteralInteger 2))
      (Variables|Default|SetStatusMessage "BİLGİ: Bu karede zaten doğru yerleştirilmiş bir KEDİ bulunuyor!")
      (CallFunction|MeowUpdateHud)
      (else
        (bind _conflictcode (CallFunction|MeowCheckConflict _row _col (Variables|/Game/23020021046/Vize/Blueprints/BP_MeowBlock.BP_MeowBlock_C|GetRegionId ClickedBlock)))
        (if (> _conflictcode (Class|KismetSystemLibrary|MakeLiteralInteger))
          (Default|MeowFlashError ClickedBlock)
          (Variables|Default|SetLives (- (Variables|Default|GetLives) (Class|KismetSystemLibrary|MakeLiteralInteger 1)))
          (if (== _conflictcode (Class|KismetSystemLibrary|MakeLiteralInteger 1))
            (Variables|Default|SetStatusMessage "KURAL İHLALİ (-1 Can): Aynı SATIRDA zaten bir kedi var! Her satırda sadece 1 kedi olabilir.")
            (elif (== _conflictcode (Class|KismetSystemLibrary|MakeLiteralInteger 2))
              (Variables|Default|SetStatusMessage "KURAL İHLALİ (-1 Can): Aynı SÜTUNDA zaten bir kedi var! Her sütunda sadece 1 kedi olabilir.")
              (elif (== _conflictcode (Class|KismetSystemLibrary|MakeLiteralInteger 3))
                (Variables|Default|SetStatusMessage "KURAL İHLALİ (-1 Can): Aynı RENK BÖLGESİNDE zaten bir kedi var! Her bölgede sadece 1 kedi olabilir.")
                (else
                  (Variables|Default|SetStatusMessage "KURAL İHLALİ (-1 Can): İki kedi birbirine temas edemez! Bir kedinin etrafındaki 8 kare (yan, üst, alt ve çaprazlar) boş kalmalıdır.")))))
          (CallFunction|MeowUpdateHud)
          (if (<= (Variables|Default|GetLives) (Class|KismetSystemLibrary|MakeLiteralInteger))
            (CallFunction|MeowTriggerGameOver))
          (elif (Utilities|Array|ContainsItem (Variables|Default|GetCurrentSolution) (Variables|/Game/23020021046/Vize/Blueprints/BP_MeowBlock.BP_MeowBlock_C|GetGridIndex ClickedBlock))
            (Default|MeowSetCellState ClickedBlock 2)
            (CallFunction|MeowApplyAutoX _row _col)
            (Variables|Default|SetCatsPlaced (+ (Variables|Default|GetCatsPlaced) (Class|KismetSystemLibrary|MakeLiteralInteger 1)))
            (Variables|Default|SetScore (+ (Variables|Default|GetScore) (Class|KismetSystemLibrary|MakeLiteralInteger 25)))
            (if (== (Variables|Default|GetCurrentLevel) (Class|KismetSystemLibrary|MakeLiteralInteger 1))
              (Variables|Default|SetStatusMessage (Utilities|Array|Get(acopy) (Variables|Default|GetTutorialPrompts) (Variables|Default|GetCatsPlaced)))
              (else
                (Variables|Default|SetStatusMessage "DOĞRU HAMLE (+25 Puan): Kedi yerleştirildi ve etrafındaki 8 komşu kare otomatik X ile işaretlendi!")))
            (CallFunction|MeowUpdateHud)
            (if (>= (Variables|Default|GetCatsPlaced) (Variables|Default|GetSize))
              (CallFunction|MeowonLevelCompleted))
            (else
              (Default|MeowFlashError ClickedBlock)
              (Variables|Default|SetLives (- (Variables|Default|GetLives) (Class|KismetSystemLibrary|MakeLiteralInteger 1)))
              (if (== (Variables|Default|GetCurrentLevel) (Class|KismetSystemLibrary|MakeLiteralInteger 1))
                (Variables|Default|SetStatusMessage "ÖĞRETİCİ UYARISI (-1 Can): Yanlış kare! Alttaki öğretici ipucunda belirtilen satır ve sütuna dikkat et.")
                (else
                  (Variables|Default|SetStatusMessage "MANTIK HATASI (-1 Can): Bu kare diğer renk bölgelerini çözümsüz bırakıyor! (İpucu için H tuşu)")))
              (CallFunction|MeowUpdateHud)
              (if (<= (Variables|Default|GetLives) (Class|KismetSystemLibrary|MakeLiteralInteger))
                (CallFunction|MeowTriggerGameOver)))))))))

(fn MeowToggleXonHovered
  (bind _hoveredblock (Variables|Default|GetHoveredBlock))
  (bind _cellstate (Variables|/Game/23020021046/Vize/Blueprints/BP_MeowBlock.BP_MeowBlock_C|GetCellState _hoveredblock))
  (if (not (or (Variables|Default|GetIsGameOver) (Variables|Default|GetIsTransitioning)))
    (Utilities|IsValid _hoveredblock
      (:Is%20Valid
        (if (== _cellstate (Class|KismetSystemLibrary|MakeLiteralInteger))
          (Default|MeowSetCellState _hoveredblock 1)
          (elif (== _cellstate (Class|KismetSystemLibrary|MakeLiteralInteger 1))
            (Default|MeowSetCellState _hoveredblock)))))))

(fn MeowUseHint
  (if (not (or (Variables|Default|GetIsGameOver) (Variables|Default|GetIsTransitioning)))
    (Variables|Default|SetHintPlacedFlag false)
    (for _array_element (Variables|Default|GetCurrentSolution)
      (if (not (Variables|Default|GetHintPlacedFlag))
        (if (!= (Variables|/Game/23020021046/Vize/Blueprints/BP_MeowBlock.BP_MeowBlock_C|GetCellState (Utilities|Array|Get(acopy) (Variables|Default|GetBlocks) _array_element)) (Class|KismetSystemLibrary|MakeLiteralInteger 2))
          (Variables|Default|SetHintPlacedFlag true)
          (Default|MeowSetCellState (Utilities|Array|Get(acopy) (Variables|Default|GetBlocks) _array_element) 2)
          (CallFunction|MeowApplyAutoX (Variables|/Game/23020021046/Vize/Blueprints/BP_MeowBlock.BP_MeowBlock_C|GetRow (Utilities|Array|Get(acopy) (Variables|Default|GetBlocks) _array_element)) (Variables|/Game/23020021046/Vize/Blueprints/BP_MeowBlock.BP_MeowBlock_C|GetCol (Utilities|Array|Get(acopy) (Variables|Default|GetBlocks) _array_element)))
          (Variables|Default|SetCatsPlaced (+ (Variables|Default|GetCatsPlaced) (Class|KismetSystemLibrary|MakeLiteralInteger 1)))
          (if (== (Variables|Default|GetCurrentLevel) (Class|KismetSystemLibrary|MakeLiteralInteger 1))
            (Variables|Default|SetStatusMessage (Utilities|Array|Get(acopy) (Variables|Default|GetTutorialPrompts) (Variables|Default|GetCatsPlaced)))
            (else
              (Variables|Default|SetStatusMessage "İPUCU (H): Doğru bir kedi yerleştirildi ve komşu kareleri [X] ile işaretlendi!")))
          (CallFunction|MeowUpdateHud)
          (if (>= (Variables|Default|GetCatsPlaced) (Variables|Default|GetSize))
            (CallFunction|MeowonLevelCompleted)))))))

(fn MeowRestartLevel
  (CallFunction|MeowLoadLevel (Variables|Default|GetCurrentLevel)))

(fn MeowLoadLevel
  (params (LevelIndex :type Integer))
  (Variables|Default|SetCurrentLevel LevelIndex)
  (Variables|Default|SetCatsPlaced 0)
  (Variables|Default|SetLives 3)
  (Variables|Default|SetIsGameOver false)
  (Variables|Default|SetIsTransitioning false)
  (Widget|SetVisibility (Variables|/Game/23020021046/Vize/UI/W_MeowHUD.W_MeowHUD_C|GettxtBanner (Variables|Default|GetHud)) "Hidden")
  (CallFunction|MeowClearBoard)
  (if (== LevelIndex (Class|KismetSystemLibrary|MakeLiteralInteger 1))
    (Variables|Default|SetSize 4)
    (Variables|Default|SetCurrentRegions (Variables|Default|GetLevel1Regions))
    (Variables|Default|SetCurrentSolution (Variables|Default|GetLevel1Solution))
    (elif (== LevelIndex (Class|KismetSystemLibrary|MakeLiteralInteger 2))
      (Variables|Default|SetSize 4)
      (Variables|Default|SetCurrentRegions (Variables|Default|GetLevel2Regions))
      (Variables|Default|SetCurrentSolution (Variables|Default|GetLevel2Solution))
      (elif (== LevelIndex (Class|KismetSystemLibrary|MakeLiteralInteger 3))
        (Variables|Default|SetSize 5)
        (Variables|Default|SetCurrentRegions (Variables|Default|GetLevel3Regions))
        (Variables|Default|SetCurrentSolution (Variables|Default|GetLevel3Solution))
        (elif (== LevelIndex (Class|KismetSystemLibrary|MakeLiteralInteger 4))
          (Variables|Default|SetSize 5)
          (Variables|Default|SetCurrentRegions (Variables|Default|GetLevel4Regions))
          (Variables|Default|SetCurrentSolution (Variables|Default|GetLevel4Solution))
          (else
            (Variables|Default|SetSize 6)
            (Variables|Default|SetCurrentRegions (Variables|Default|GetLevel5Regions))
            (Variables|Default|SetCurrentSolution (Variables|Default|GetLevel5Solution)))))))
  (Variables|Default|SetStatusMessage (Utilities|Array|Get(acopy) (Variables|Default|GetLevelPrompts) LevelIndex))
  (bind _returnvalue (Actor|GetActorOfClass "/Script/Engine.CameraActor"))
  (Transformation|SetActorLocation _returnvalue (Math|Vector|MakeVector (* (* (Math|Conversions|ToFloat(Integer) (- (Variables|Default|GetSize) (Class|KismetSystemLibrary|MakeLiteralInteger 1))) (Variables|Default|GetSpacing)) (Math|Float|MakeLiteralFloat 0.5)) (* (* (Math|Conversions|ToFloat(Integer) (- (Variables|Default|GetSize) (Class|KismetSystemLibrary|MakeLiteralInteger 1))) (Variables|Default|GetSpacing)) (Math|Float|MakeLiteralFloat 0.5)) (+ (Math|Float|MakeLiteralFloat 4.5e+02) (* (Math|Conversions|ToFloat(Integer) (Variables|Default|GetSize)) (Math|Float|MakeLiteralFloat 3e+02)))) false false)
  (for _index (range 0 (- (Variables|Default|GetSize) (Class|KismetSystemLibrary|MakeLiteralInteger 1)))
    (for _index_2 (range 0 (- (Variables|Default|GetSize) (Class|KismetSystemLibrary|MakeLiteralInteger 1)))
      (CallFunction|MeowCreateBlock _index _index_2)))
  (CallFunction|MeowUpdateHud))

(fn MeowClearBoard
  (bind _blocks (Variables|Default|GetBlocks))
  (for _array_element _blocks
    (Utilities|IsValid _array_element
      (:Is%20Valid
        (Actor|DestroyActor _array_element))))
  (Utilities|Array|Clear _blocks))

(fn MeowUpdateHud
  (bind _hud (Variables|Default|GetHud))
  (Utilities|IsValid _hud
    (:Is%20Valid
      (Rendering|Components|TextRender|SetText (Variables|/Game/23020021046/Vize/UI/W_MeowHUD.W_MeowHUD_C|GettxtLevel _hud) (Utilities|Text|ToText(String) (Utilities|Array|Get(acopy) (Variables|Default|GetLevelTitles) (Variables|Default|GetCurrentLevel))))
      (Rendering|Components|TextRender|SetText (Variables|/Game/23020021046/Vize/UI/W_MeowHUD.W_MeowHUD_C|GettxtCats _hud) (Utilities|Text|ToText(String) (Utilities|String|Append (Utilities|String|Append "Kediler: " (Utilities|String|ToString(Integer) (Variables|Default|GetCatsPlaced))) (Utilities|String|Append " / " (Utilities|String|ToString(Integer) (Variables|Default|GetSize))))))
      (Rendering|Components|TextRender|SetText (Variables|/Game/23020021046/Vize/UI/W_MeowHUD.W_MeowHUD_C|GettxtLives _hud) (Utilities|Text|ToText(String) (Utilities|String|Append "Can: " (Utilities|String|Append (Utilities|String|ToString(Integer) (Variables|Default|GetLives)) " / 3"))))
      (Rendering|Components|TextRender|SetText (Variables|/Game/23020021046/Vize/UI/W_MeowHUD.W_MeowHUD_C|GettxtScore _hud) (Utilities|Text|ToText(String) (Utilities|String|Append "Puan: " (Utilities|String|ToString(Integer) (Variables|Default|GetScore)))))
      (Rendering|Components|TextRender|SetText (Variables|/Game/23020021046/Vize/UI/W_MeowHUD.W_MeowHUD_C|GettxtTutorial _hud) (Utilities|Text|ToText(String) (Variables|Default|GetStatusMessage))))))

(fn MeowCreateBlock
  (params (InRow :type Integer) (InCol :type Integer))
  (bind _size (Variables|Default|GetSize))
  (bind _spacing (Variables|Default|GetSpacing))
  (bind _returnvalue (* InRow _size))
  (bind _returnvalue_2 (+ _returnvalue InCol))
  (bind _returnvalue_3 (Game|SpawnActorfromClass "/Game/23020021046/Vize/Blueprints/BP_MeowBlock.BP_MeowBlock_C" (Math|Transform|MakeTransform (+ (Transformation|GetActorLocation) (Math|Vector|MakeVector (* (Math|Conversions|ToFloat(Integer) (- (- _size (Class|KismetSystemLibrary|MakeLiteralInteger 1)) InRow)) _spacing) (* (Math|Conversions|ToFloat(Integer) InCol) _spacing) 0.0))) "AlwaysSpawn" "MultiplyWithRoot" 0 0))
  (Default|MeowInitBlock _returnvalue_3 self _returnvalue_2 InRow InCol (Utilities|Array|Get(acopy) (Variables|Default|GetCurrentRegions) _returnvalue_2))
  (Utilities|Array|SetArrayElem (Variables|Default|GetBlocks) _returnvalue_2 _returnvalue_3 true))

(fn MeowApplyAutoX
  (params (CatRow :type Integer) (CatCol :type Integer))
  (for _array_element (Variables|Default|GetBlocks)
    (if (== (Variables|/Game/23020021046/Vize/Blueprints/BP_MeowBlock.BP_MeowBlock_C|GetCellState _array_element) (Class|KismetSystemLibrary|MakeLiteralInteger))
      (if (and (<= (Math|Integer|Absolute(Integer) (- (Variables|/Game/23020021046/Vize/Blueprints/BP_MeowBlock.BP_MeowBlock_C|GetRow _array_element) CatRow)) (Class|KismetSystemLibrary|MakeLiteralInteger 1)) (<= (Math|Integer|Absolute(Integer) (- (Variables|/Game/23020021046/Vize/Blueprints/BP_MeowBlock.BP_MeowBlock_C|GetCol _array_element) CatCol)) (Class|KismetSystemLibrary|MakeLiteralInteger 1)))
        (Default|MeowSetCellState _array_element 1)))))

(fn MeowCheckConflict
  (params (TargetRow :type Integer) (TargetCol :type Integer) (TargetRegion :type Integer))
  (Variables|Default|SetLastConflictCode 0)
  (for _array_element (Variables|Default|GetBlocks)
    (if (== (Variables|/Game/23020021046/Vize/Blueprints/BP_MeowBlock.BP_MeowBlock_C|GetCellState _array_element) (Class|KismetSystemLibrary|MakeLiteralInteger 2))
      (if (== (Variables|/Game/23020021046/Vize/Blueprints/BP_MeowBlock.BP_MeowBlock_C|GetRow _array_element) TargetRow)
        (Variables|Default|SetLastConflictCode 1)
        (elif (== (Variables|/Game/23020021046/Vize/Blueprints/BP_MeowBlock.BP_MeowBlock_C|GetCol _array_element) TargetCol)
          (Variables|Default|SetLastConflictCode 2)
          (elif (== (Variables|/Game/23020021046/Vize/Blueprints/BP_MeowBlock.BP_MeowBlock_C|GetRegionId _array_element) TargetRegion)
            (Variables|Default|SetLastConflictCode 3)
            (elif (and (<= (Math|Integer|Absolute(Integer) (- (Variables|/Game/23020021046/Vize/Blueprints/BP_MeowBlock.BP_MeowBlock_C|GetRow _array_element) TargetRow)) (Class|KismetSystemLibrary|MakeLiteralInteger 1)) (<= (Math|Integer|Absolute(Integer) (- (Variables|/Game/23020021046/Vize/Blueprints/BP_MeowBlock.BP_MeowBlock_C|GetCol _array_element) TargetCol)) (Class|KismetSystemLibrary|MakeLiteralInteger 1)))
              (Variables|Default|SetLastConflictCode 4)))))))
  (return (Variables|Default|GetLastConflictCode)))

(fn MeowToggleXonBlock
  (params (TargetBlock :type BP%20Meow%20Block%20Object%20Reference))
  (bind _cellstate (Variables|/Game/23020021046/Vize/Blueprints/BP_MeowBlock.BP_MeowBlock_C|GetCellState TargetBlock))
  (if (not (or (Variables|Default|GetIsGameOver) (Variables|Default|GetIsTransitioning)))
    (Utilities|IsValid TargetBlock
      (:Is%20Valid
        (if (== _cellstate (Class|KismetSystemLibrary|MakeLiteralInteger))
          (Default|MeowSetCellState TargetBlock 1)
          (elif (== _cellstate (Class|KismetSystemLibrary|MakeLiteralInteger 1))
            (Default|MeowSetCellState TargetBlock)))))))