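; BP_MeowBlock is one clickable tile of a cat-placement grid puzzle, initialized by its grid with index, row, column and region.
; Clicks and hovers report to MeowGrid, and hovering also enlarges the block.
; MeowSetCellState applies the region material and shows the region letter, a cross, or a raised cat head labeled "KEDI".
; MeowFlashError briefly swaps in an error material before restoring the region one.
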(event OnClicked(Block)
  (params (TouchedComponent :type Primitive%20Component%20Object%20Reference) (ButtonPressed :type Key%20Structure))
  (Default|MeowonTileLeftClicked (Variables|Default|GetMeowGrid) self))

(event OnBeginCursorOver(Block)
  (params (TouchedComponent :type Primitive%20Component%20Object%20Reference))
  (Transformation|SetRelativeScale3D (Variables|Default|GetBlock) (Math|Vector|MakeVector 2.65 2.65 0.25))
  (Default|MeowSetHoveredBlock (Variables|Default|GetMeowGrid) self))

(event OnEndCursorOver(Block)
  (params (TouchedComponent :type Primitive%20Component%20Object%20Reference))
  (Transformation|SetRelativeScale3D (Variables|Default|GetBlock) (Math|Vector|MakeVector 2.45 2.45 0.25)))

(event Custom|MeowFlashError
  (bind _block (Variables|Default|GetBlock))
  (Rendering|Material|SetMaterial _block 0 "/Game/23020021046/Vize/Materials/MI_Error.MI_Error")
  (Utilities|FlowControl|Delay 0.45)
  (Rendering|Material|SetMaterial _block 0 (Utilities|Array|Get(acopy) (Variables|Default|GetRegionMaterials) (Variables|Default|GetRegionId))))

(event EventBeginPlay)

(event Collision|EventActorBeginOverlap
  (params (OtherActor :type Actor%20Object%20Reference)))

(event EventTick
  (params (DeltaSeconds :type Float%20%28single-precision%29)))

(fn ConstructionScript)

(fn MeowSetCellState
  (params (NewState :type Integer))
  (bind _block (Variables|Default|GetBlock))
  (bind _cathead (Variables|Default|GetCatHead))
  (bind _crossroot (Variables|Default|GetCrossRoot))
  (bind _label (Variables|Default|GetLabel))
  (bind _regionid (Variables|Default|GetRegionId))
  (Variables|Default|SetCellState NewState)
  (Rendering|Material|SetMaterial _block 0 (Utilities|Array|Get(acopy) (Variables|Default|GetRegionMaterials) _regionid))
  (if (== NewState (Class|KismetSystemLibrary|MakeLiteralInteger 2))
    (Rendering|SetVisibility _cathead true true)
    (Rendering|SetVisibility _crossroot false true)
    (Rendering|SetVisibility _label true false)
    (Transformation|SetRelativeLocation _block (Math|Vector|MakeVector 0.0 0.0 18.0) false false)
    (Transformation|SetRelativeLocation _label (Math|Vector|MakeVector -75.0 0.0 36.0) false false)
    (Rendering|Components|TextRender|SetText _label (Utilities|Text|ToText(String) "KEDI"))
    (elif (== NewState (Class|KismetSystemLibrary|MakeLiteralInteger 1))
      (Rendering|SetVisibility _cathead false true)
      (Rendering|SetVisibility _crossroot true true)
      (Rendering|SetVisibility _label false false)
      (Transformation|SetRelativeLocation _block (Math|Vector|MakeVector 0.0 0.0 0.0) false false)
      (else
        (Rendering|SetVisibility _cathead false true)
        (Rendering|SetVisibility _crossroot false true)
        (Rendering|SetVisibility _label true false)
        (Transformation|SetRelativeLocation _block (Math|Vector|MakeVector 0.0 0.0 0.0) false false)
        (Transformation|SetRelativeLocation _label (Math|Vector|MakeVector 0.0 0.0 18.0) false false)
        (Rendering|Components|TextRender|SetText _label (Utilities|Text|ToText(String) (Utilities|Array|Get(acopy) (Variables|Default|GetRegionLetters) _regionid)))))))

(fn MeowInitBlock
  (params (InGrid :type BP%20Meow%20Grid%20Object%20Reference) (InIndex :type Integer) (InRow :type Integer) (InCol :type Integer) (InRegion :type Integer))
  (Variables|Default|SetMeowGrid InGrid)
  (Variables|Default|SetGridIndex InIndex)
  (Variables|Default|SetRow InRow)
  (Variables|Default|SetCol InCol)
  (Variables|Default|SetRegionId InRegion)
  (CallFunction|MeowSetCellState))