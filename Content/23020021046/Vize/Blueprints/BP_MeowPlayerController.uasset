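; Player controller for a grid puzzle game that turns mouse and keyboard input into commands on the BP_MeowGrid actor.
; On BeginPlay it sets Game and UI input mode and switches the view to a CameraActor in the level.
; Right-click or X toggles an X mark on the BP_MeowBlock under the cursor, falling back to the grid's hovered block.
; Other keys trigger a hint, restart the level, or load one of five levels.
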(event Custom|OnRightClick
  (bind _self self)
  (bind (_hitresult _returnvalue) (Game|Player|GetHitResultUnderCursorbyChannel _self "TraceTypeQuery1" false))
  (bind _returnvalue_2 (Actor|GetActorOfClass "/Game/23020021046/Vize/Blueprints/BP_MeowGrid.BP_MeowGrid_C"))
  (if _returnvalue
    (bind _asbp_meow_block (Utilities|Casting|CastToBP_MeowBlock (.HitActor (Collision|BreakHitResult _hitresult)))
      (:then
        (Default|MeowToggleXonBlock _returnvalue_2 _asbp_meow_block))
      (:CastFailed
        (Default|MeowToggleXonHovered _returnvalue_2)))
    (else
      (Default|MeowToggleXonHovered _returnvalue_2))))

(event Custom|OnHintKey
  (bind _returnvalue (Actor|GetActorOfClass "/Game/23020021046/Vize/Blueprints/BP_MeowGrid.BP_MeowGrid_C"))
  (Default|MeowUseHint _returnvalue))

(event Custom|OnRestartKey
  (bind _returnvalue (Actor|GetActorOfClass "/Game/23020021046/Vize/Blueprints/BP_MeowGrid.BP_MeowGrid_C"))
  (Default|MeowRestartLevel _returnvalue))

(event Custom|OnLevel1Key
  (bind _returnvalue (Actor|GetActorOfClass "/Game/23020021046/Vize/Blueprints/BP_MeowGrid.BP_MeowGrid_C"))
  (Default|MeowLoadLevel _returnvalue 1))

(event Custom|OnLevel2Key
  (bind _returnvalue (Actor|GetActorOfClass "/Game/23020021046/Vize/Blueprints/BP_MeowGrid.BP_MeowGrid_C"))
  (Default|MeowLoadLevel _returnvalue 2))

(event Custom|OnLevel3Key
  (bind _returnvalue (Actor|GetActorOfClass "/Game/23020021046/Vize/Blueprints/BP_MeowGrid.BP_MeowGrid_C"))
  (Default|MeowLoadLevel _returnvalue 3))

(event Custom|OnLevel4Key
  (bind _returnvalue (Actor|GetActorOfClass "/Game/23020021046/Vize/Blueprints/BP_MeowGrid.BP_MeowGrid_C"))
  (Default|MeowLoadLevel _returnvalue 4))

(event Custom|OnLevel5Key
  (bind _returnvalue (Actor|GetActorOfClass "/Game/23020021046/Vize/Blueprints/BP_MeowGrid.BP_MeowGrid_C"))
  (Default|MeowLoadLevel _returnvalue 5))

(event EventBeginPlay
  (bind _self self)
  (Input|SetInputModeGameandUI _self 0 "DoNotLock" false false)
  (bind _returnvalue (Actor|GetActorOfClass "/Script/Engine.CameraActor"))
  (Game|Player|SetViewTargetwithBlend _self _returnvalue 0.0 "VTBlend_Linear" 0.0 false))

(event EventTick
  (params (DeltaSeconds :type Float%20%28single-precision%29)))

(event Input|MouseEvents|RightMouseButton
  (params (Key :type Key%20Structure))
  (:Pressed
    (CallFunction|OnRightClick)))

(event Input|KeyboardEvents|X
  (params (Key :type Key%20Structure))
  (:Pressed
    (CallFunction|OnRightClick)))

(event Input|KeyboardEvents|H
  (params (Key :type Key%20Structure))
  (:Pressed
    (CallFunction|OnHintKey)))

(event Input|KeyboardEvents|R
  (params (Key :type Key%20Structure))
  (:Pressed
    (CallFunction|OnRestartKey)))

(event Input|KeyboardEvents|1
  (params (Key :type Key%20Structure))
  (:Pressed
    (CallFunction|OnLevel1Key)))

(event Input|KeyboardEvents|2
  (params (Key :type Key%20Structure))
  (:Pressed
    (CallFunction|OnLevel2Key)))

(event Input|KeyboardEvents|3
  (params (Key :type Key%20Structure))
  (:Pressed
    (CallFunction|OnLevel3Key)))

(event Input|KeyboardEvents|4
  (params (Key :type Key%20Structure))
  (:Pressed
    (CallFunction|OnLevel4Key)))

(event Input|KeyboardEvents|5
  (params (Key :type Key%20Structure))
  (:Pressed
    (CallFunction|OnLevel5Key)))

(fn ConstructionScript)